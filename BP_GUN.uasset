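; BP_GUN is a motion-controller VR gun that supports one- or two-handed holding and destroys enemies.
; Pickup and Drop toggle physics and attachment to the first controller.
; A second controller overlapping SecondHandTrigger makes Tick aim the gun between both hands, keeping first-hand roll, until that overlap ends, subject to grip state.
; GripRight fires, without checking whether held: an explosion effect, sound and line trace that destroys any EnemyCharacter_BP hit.
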(event `InputAction|GripRight`
  (params (Key :type "Key Structure"))
  (bind _arrow (`self.Arrow`))
  (bind _returnvalue (`SceneComponent.K2_GetComponentLocation` _arrow))
  (:`Pressed`
    (bind _outhit (`KismetSystemLibrary.LineTraceSingle` _returnvalue (+ _returnvalue (* (`SceneComponent.GetForwardVector` _arrow) 1000)) "TraceTypeQuery1"))
    (`GameplayStatics.SpawnEmitterAtLocation` "/Game/StarterContent/Particles/P_Explosion.P_Explosion" _returnvalue)
    (`GameplayStatics.PlaySound2D` "/Game/StarterContent/Audio/Explosion02.Explosion02" 1.0 1.0 0.0 null null)
    (bind _asenemy_character_bp (cast `/Game/EnemyCharacter_BP` (`.HitActor` (`GameplayStatics.BreakHitResult` _outhit))))
    (`self.K2_DestroyActor` _asenemy_character_bp)))

(event `/Game/VirtualRealityBP/Blueprints/PickupActorInterface.Pickup`
  (params (AttachTo :type "SceneComponent Object Reference"))
  (if (not (`self.bIsFirstHandAttached`))
    (`PrimitiveComponent.SetSimulatePhysics` (`self.StaticMeshComponent`) false)
    (`SceneComponent.K2_AttachToComponent` (`self.K2_GetRootComponent`) AttachTo "None" "SnapToTarget" "SnapToTarget" "KeepWorld" false)
    (`SceneComponent.K2_SetRelativeRotation` (`self.StaticMeshComponent`) (`self.OneHandRotation`) false false)
    (set `self.bIsFirstHandAttached` true)
    (set `self.bIsSecondHandTrackingActive` false)
    (set `self.FirstHand` AttachTo)))

(event `/Game/VirtualRealityBP/Blueprints/PickupActorInterface.Drop`
  (`PrimitiveComponent.SetSimulatePhysics` (`self.StaticMeshComponent`) true)
  (`self.K2_DetachFromActor` "KeepWorld" "KeepWorld" "KeepWorld")
  (set `self.bIsFirstHandAttached` false)
  (set `self.bIsSecondHandTrackingActive` false))

(event `self.SecondHandTrigger.OnComponentBeginOverlap`
  (params (OverlappedComponent :type "PrimitiveComponent Object Reference") (OtherActor :type "Actor Object Reference") (OtherComp :type "PrimitiveComponent Object Reference") (OtherBodyIndex :type Integer) (bFromSweep :type Boolean) (SweepResult :type "HitResult Structure (by ref)"))
  (if (`self.bIsFirstHandAttached`)
    (bind _asbp_motion_controller (cast `/Game/VirtualRealityBP/Blueprints/BP_MotionController` OtherActor))
    (bind _motioncontroller (`/Game/VirtualRealityBP/Blueprints/BP_MotionController.MotionController` _asbp_motion_controller))
    (if (!= (`self.FirstHand`) _motioncontroller)
      (set `self.bIsSecondHandTrackingActive` true)
      (set `self.SecondHand` _motioncontroller))))

(event `self.2ndHandTrigger.OnComponentBeginOverlap`
  (params (OverlappedComponent :type "PrimitiveComponent Object Reference") (OtherActor :type "Actor Object Reference") (OtherComp :type "PrimitiveComponent Object Reference") (OtherBodyIndex :type Integer) (bFromSweep :type Boolean) (SweepResult :type "HitResult Structure (by ref)")))

(event `self.SecondHandTrigger.OnComponentEndOverlap`
  (params (OverlappedComponent :type "PrimitiveComponent Object Reference") (OtherActor :type "Actor Object Reference") (OtherComp :type "PrimitiveComponent Object Reference") (OtherBodyIndex :type Integer))
  (bind (_asbp_motion_controller _bsuccess) (cast `/Game/VirtualRealityBP/Blueprints/BP_MotionController` (`ActorComponent.GetOwner` (`self.SecondHand`)) :!pure true))
  (if (`self.bIsSecondHandTrackingActive`)
    (`/Engine/EditorBlueprintResources/StandardMacros.IsValid` (`self.SecondHand`)
      (:`Is Valid`
        (if (and (`|EnumInequality` (`/Game/VirtualRealityBP/Blueprints/BP_MotionController.GripState` _asbp_motion_controller) "NewEnumerator2") _bsuccess)
          (set `self.bIsSecondHandTrackingActive` false :!label _label)
          (set `self.SecondHand` null)
          (`SceneComponent.K2_SetRelativeRotation` (`self.StaticMeshComponent`) (`self.OneHandRotation`) false false)))
      (:`Is Not Valid`
        (goto _label)))))

(event `self.2ndHandTrigger.OnComponentEndOverlap`
  (params (OverlappedComponent :type "PrimitiveComponent Object Reference") (OtherActor :type "Actor Object Reference") (OtherComp :type "PrimitiveComponent Object Reference") (OtherBodyIndex :type Integer)))

(event `self.ReceiveTick`
  (params (DeltaSeconds :type "Float (single-precision)"))
  (bind _firsthand (`self.FirstHand`))
  (if (and (`self.bIsSecondHandTrackingActive`) (`KismetSystemLibrary.IsValid` (`self.SecondHand`)))
    (`SceneComponent.K2_SetWorldRotation` (`self.StaticMeshComponent`) (`KismetMathLibrary.MakeRotator` (.roll (`SceneComponent.K2_GetComponentRotation` _firsthand)) (.pitch (`KismetMathLibrary.FindLookAtRotation` (`SceneComponent.K2_GetComponentLocation` _firsthand) (`SceneComponent.K2_GetComponentLocation` (`self.SecondHand`)))) (.yaw (`KismetMathLibrary.FindLookAtRotation` (`SceneComponent.K2_GetComponentLocation` _firsthand) (`SceneComponent.K2_GetComponentLocation` (`self.SecondHand`))))) false false)))

(fn `UserConstructionScript`)